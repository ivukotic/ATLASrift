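; A stripped-down LHC magnet exhibit in the detector cavern, with two overlap-triggered controls.
; The switch toggles visibility of the Magnets component and shifts itself for five seconds, using a DoOnce to block retriggering until it returns.
; The tour trigger saves the player pawn's location in the ATLAS game instance, then opens ControlRoomLevel with an LHC magnets option.
; Both play a clink at the world origin and print a debug message.
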(event OnComponentBeginOverlap(LHCmagnet-tour)
  (params (OverlappedComponent :type Primitive%20Component%20Object%20Reference) (OtherActor :type Actor%20Object%20Reference) (OtherComp :type Primitive%20Component%20Object%20Reference) (OtherBodyIndex :type Integer) (bFromSweep :type Boolean) (SweepResult :type Hit%20Result%20Structure%20%28by%20ref%29))
  (Audio|PlaySoundatLocation "/Game/StarterContent/Audio/clink.clink" "0, 0, 0")
  (Development|PrintString "Magnets to Tour")
  (bind _asatlasgame_instance (Utilities|Casting|CastToATLASGameInstance (Game|GetGameInstance)))
  (Default|SetPlayerLocation _asatlasgame_instance 0 (Transformation|GetActorLocation (Game|Player|GetPlayerPawn 0)))
  (Game|OpenLevel(byName) "ControlRoomLevel" false "LHC_magnets"))

(event OnComponentBeginOverlap(LHCmagnet-switch)
  (params (OverlappedComponent :type Primitive%20Component%20Object%20Reference) (OtherActor :type Actor%20Object%20Reference) (OtherComp :type Primitive%20Component%20Object%20Reference) (OtherBodyIndex :type Integer) (bFromSweep :type Boolean) (SweepResult :type Hit%20Result%20Structure%20%28by%20ref%29))
  (Utilities|FlowControl|DoOnce false :!label _label
    (:Completed
      (Audio|PlaySoundatLocation "/Game/StarterContent/Audio/clink.clink" "0, 0, 0")
      (Development|PrintString "Toggling  magnets")
      (Rendering|ToggleVisibility (Variables|Default|GetMagnets) false)
      (Transformation|AddLocalOffset (Variables|Default|GetLHCmagnet-switch) "-8.000000, 0, 0" false false)
      (Utilities|FlowControl|Delay 5.0)
      (Transformation|AddLocalOffset (Variables|Default|GetLHCmagnet-switch) "8.000000, 0, 0" false false)
      (goto _label Reset))))

(event EventBeginPlay)

(event Collision|EventActorBeginOverlap
  (params (OtherActor :type Actor%20Object%20Reference)))

(event EventTick
  (params (DeltaSeconds :type Float%20%28single-precision%29)))

(fn ConstructionScript)