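; DetectorBP controls how one subdetector mesh is displayed: solid, wireframe, transparent or hidden.
; SetMesh stores the mesh and caches its original materials, which solid mode restores.
; Wireframe and transparent modes override every material slot with a shared material, while hidden mode hides the mesh and its children.
; ShiftState cycles through the four modes and applies each through the SetVisualization event.
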(event Custom|SetVisualization
  (params (NewVisualization :type DetectorVisualization%20Enum :default "NewEnumerator0"))
  (switch Utilities|FlowControl|Switch|SwitchonDetectorVisualization NewVisualization
    (:NewEnumerator0
      (CallFunction|MakeSolid))
    (:NewEnumerator1
      (CallFunction|MakeWireframe))
    (:NewEnumerator2
      (CallFunction|MakeTransluscent))
    (:NewEnumerator3
      (CallFunction|MakeInvisible))))

(fn MakeSolid
  (bind _subdetmesh (Variables|Default|GetsubdetMesh))
  (Variables|Default|SetState "NewEnumerator0")
  (CallFunction|MakeVisible)
  (for (_ _array_index) (Rendering|Material|GetMaterials _subdetmesh)
    (Rendering|Material|SetMaterial _subdetmesh _array_index (Utilities|Array|Get(acopy) (Variables|Default|Getmats) _array_index)))
  (Development|PrintString (Utilities|String|Append "Made subdetector solid: " (Utilities|GetObjectName _subdetmesh)) false))

(fn MakeInvisible
  (bind _subdetmesh (Variables|Default|GetsubdetMesh))
  (Variables|Default|SetState "NewEnumerator3")
  (Development|SetHiddeninGame _subdetmesh true true)
  (Development|PrintString (Utilities|String|Append "Made subdetector invisible:  " (Utilities|GetObjectName _subdetmesh)) false))

(fn ShiftState
  (bind _output_get (Variables|Default|SetState (Utilities|Enum|ByteToEnumDetectorVisualization (Math|Conversions|ToByte(Integer) (Math|Integer|%(Integer) (+ (Math|Conversions|ToInteger(Byte) (Variables|Default|GetState)) 1) 4)))))
  (CallFunction|SetVisualization _output_get))

(fn MakeTransluscent
  (bind _subdetmesh (Variables|Default|GetsubdetMesh))
  (Variables|Default|SetState "NewEnumerator2")
  (CallFunction|MakeVisible)
  (for (_ _array_index) (Rendering|Material|GetMaterials _subdetmesh)
    (Rendering|Material|SetMaterial _subdetmesh _array_index "/Game/Materials/M_Glass.M_Glass"))
  (Development|PrintString (Utilities|String|Append "Made subdetector transluscent:  " (Utilities|GetObjectName _subdetmesh))))

(fn MakeWireframe
  (bind _subdetmesh (Variables|Default|GetsubdetMesh))
  (Variables|Default|SetState "NewEnumerator1")
  (CallFunction|MakeVisible)
  (for (_ _array_index) (Rendering|Material|GetMaterials _subdetmesh)
    (Rendering|Material|SetMaterial _subdetmesh _array_index "/Game/Materials/WRFR.WRFR"))
  (Development|PrintString (Utilities|String|Append "Made subdetector wireframe :   " (Utilities|GetObjectName _subdetmesh))))

(fn SetMesh
  (params (mesh :type Static%20Mesh%20Component%20Object%20Reference))
  (bind _output_get (Variables|Default|SetsubdetMesh mesh))
  (Variables|Default|Setmats (Rendering|Material|GetMaterials _output_get)))

(fn MakeVisible
  (Development|SetHiddeninGame (Variables|Default|GetsubdetMesh) false true))