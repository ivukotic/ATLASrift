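; DetectorBP controls how one detector subdetector mesh is displayed: solid, invisible, translucent, wireframe or solo.
; SetMesh stores the mesh and its original materials, which Solid restores, while Translucent and Wireframe override every material slot.
; ShiftState cycles the five states through ShowItAs, which plays a switch sound and dispatches to the matching function.
; Solo unhides the mesh and messages tagged actors whose first tag differs from its owner's to turn invisible.
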(event EventBeginPlay)

(event EventTick
  (params (DeltaSeconds :type Float%20%28single-precision%29)))

(fn MakeSolid
  (bind _subdetmesh (Variables|Default|GetsubdetMesh))
  (Variables|Default|SetcurrentState 0)
  (CallFunction|MakeVisible)
  (for (_ _array_index) (Rendering|Material|GetMaterials _subdetmesh)
    (Rendering|Material|SetMaterial _subdetmesh _array_index (Utilities|Array|Get(acopy) (Variables|Default|Getmats) _array_index)))
  (Development|PrintString (Utilities|String|Append "Made subdetector solid: " (Utilities|GetObjectName _subdetmesh))))

(fn MakeInvisible
  (bind _subdetmesh (Variables|Default|GetsubdetMesh))
  (Variables|Default|SetcurrentState 1)
  (Development|SetHiddeninGame _subdetmesh true true)
  (Development|PrintString (Utilities|String|Append "Made subdetector invisible:  " (Utilities|GetObjectName _subdetmesh)) false))

(fn ShiftState
  (bind _output_get (Variables|Default|SetcurrentState (Math|Integer|%(Integer) (+ (Variables|Default|GetcurrentState) 1) 5)))
  (CallFunction|ShowItas (Utilities|Array|Get(acopy) (Variables|Default|Getstates) _output_get)))

(fn MakeTransluscent
  (bind _subdetmesh (Variables|Default|GetsubdetMesh))
  (Variables|Default|SetcurrentState 2)
  (CallFunction|MakeVisible)
  (for (_ _array_index) (Rendering|Material|GetMaterials _subdetmesh)
    (Rendering|Material|SetMaterial _subdetmesh _array_index "/Game/Materials/M_Glass.M_Glass"))
  (Development|PrintString (Utilities|String|Append "Made subdetector transluscent:  " (Utilities|GetObjectName _subdetmesh))))

(fn MakeWireframe
  (bind _subdetmesh (Variables|Default|GetsubdetMesh))
  (Variables|Default|SetcurrentState 3)
  (CallFunction|MakeVisible)
  (for (_ _array_index) (Rendering|Material|GetMaterials _subdetmesh)
    (Rendering|Material|SetMaterial _subdetmesh _array_index "/Game/Materials/WRFR.WRFR"))
  (Development|PrintString (Utilities|String|Append "Made subdetector wireframe :   " (Utilities|GetObjectName _subdetmesh))))

(fn MakeSolo
  (Variables|Default|SetcurrentState 4)
  (CallFunction|MakeVisible)
  (Development|PrintString (Utilities|String|Append "Making subdetector solo :   " (Utilities|GetObjectName (Components|GetOwner (Variables|Default|GetsubdetMesh)))) false)
  (bind _outactors (Actor|GetAllActorsOfClass "/Script/Engine.Actor"))
  (for _array_element _outactors
    (if (> (Utilities|Array|Length (Variables|/Script/Engine.Actor|GetTags _array_element)) 0)
      (if (not (Utilities|Name|Equal(Name) (Utilities|Array|Get(acopy) (Variables|/Script/Engine.Actor|GetTags _array_element)) (Utilities|Array|Get(acopy) (Variables|/Script/Engine.Actor|GetTags (Components|GetOwner (Variables|Default|GetsubdetMesh))))))
        (Class|SubDetInterface|ShowItas(Message) _array_element "invisible"))))
  (Development|PrintString "Making SOLO DONE!" false))

(fn SetMesh
  (params (mesh :type Static%20Mesh%20Component%20Object%20Reference))
  (bind _output_get (Variables|Default|SetsubdetMesh mesh))
  (Variables|Default|Setmats (Rendering|Material|GetMaterials _output_get)))

(fn MakeVisible
  (Development|SetHiddeninGame (Variables|Default|GetsubdetMesh) false true))

(fn ShowItas
  (params (visualization :type String))
  (Audio|PlaySoundatLocation "/Game/Audio/switch-13.switch-13" "0, 0, 0" "0, 0, 0" 1.0)
  (switch string visualization
    (:solid
      (CallFunction|MakeSolid))
    (:invisible
      (CallFunction|MakeInvisible))
    (:translucent
      (CallFunction|MakeTransluscent))
    (:wireframe
      (CallFunction|MakeWireframe))
    (:solo
      (CallFunction|MakeSolo))))