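; EventBP is a particle-collision event display that shows downloaded events with event and run numbers.
; Next, previous or the F key changes EventID and calls UpdateEvent to fetch data; OnEventDownloaded then triggers DrawEvent.
; Clusters and tracks become procedural mesh sections with separate materials, with visibility toggles for both and for Jet actors.
; ClearPreviousEvent's actor cleanup is disconnected, and auto-reload toggling schedules one delayed, non-looping update.
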(event EventToggleTracks
  (Rendering|ToggleVisibility (Variables|Default|GetTrackComponent) false))

(event EventToggleJets
  (CallFunction|LToggleJets))

(event EventToggleClusters
  (Rendering|ToggleVisibility (Variables|Default|GetClusterComponent) false))

(event EventLoadPrevious
  (CallFunction|LLoadPrevious))

(event EventLoadNext
  (CallFunction|LLoadNext))

(event EventOnEventDownloaded
  (CallFunction|DrawEvent))

(event EventToggleAutoLoad
  (Variables|Default|SetEventState (Utilities|Struct|MakeEventState (.ShowTracks (Utilities|Struct|BreakEventState (Variables|Default|GetEventState))) (.ShowJets (Utilities|Struct|BreakEventState (Variables|Default|GetEventState))) (.ShowClusters (Utilities|Struct|BreakEventState (Variables|Default|GetEventState))) (not (.AutoReload (Utilities|Struct|BreakEventState (Variables|Default|GetEventState)))) (.ChangeToPreviousEvent (Utilities|Struct|BreakEventState (Variables|Default|GetEventState))) (.ChangeToNextEvent (Utilities|Struct|BreakEventState (Variables|Default|GetEventState)))))
  (Development|PrintString "Auto RELOAD is set to " false)
  (Development|PrintString (Utilities|String|ToString(Boolean) (not (.AutoReload (Utilities|Struct|BreakEventState (Variables|Default|GetEventState))))) false)
  (Utilities|Time|SetTimerbyFunctionName 0 "UpdateEvent" 5.0))

(event Input|KeyboardEvents|F
  (params (Key :type Key%20Structure :default "AnyKey"))
  (:Pressed
    (Development|SetHiddeninGame (Variables|Default|GetScene) false true)
    (CallFunction|LLoadNext)))

(fn ConstructionScript)

(fn ShowClusters
  (Class|Event|ShowClustersFunc)
  (Class|ProceduralMeshComponent|CreateMeshSection (Variables|Default|GetClusterComponent) 0 (Variables|Default|GetVertices) (Variables|Default|GetTriangles) 0 0 0 0 false)
  (Rendering|Material|SetMaterial (Variables|Default|GetClusterComponent) 0 "/Game/Materials/M_Metal_Yellow.M_Metal_Yellow"))

(fn LToggleJets
  (Development|PrintString "Toggle Jets!" false)
  (bind _outactors (Actor|GetAllActorsOfClass "/Script/ATLASrift.Jet"))
  (for _array_element _outactors
    (Rendering|ToggleVisibility (Utilities|Array|Get(acopy) (Actor|GetComponentsByClass _array_element "/Script/Engine.StaticMeshComponent")) false)))

(fn LLoadPrevious
  (Development|PrintString "Loading previous !")
  (Variables|Default|SetEventState (Utilities|Struct|MakeEventState (.ShowTracks (Utilities|Struct|BreakEventState (Variables|Default|GetEventState))) (.ShowJets (Utilities|Struct|BreakEventState (Variables|Default|GetEventState))) (.ShowClusters (Utilities|Struct|BreakEventState (Variables|Default|GetEventState))) (.AutoReload (Utilities|Struct|BreakEventState (Variables|Default|GetEventState))) true (.ChangeToNextEvent (Utilities|Struct|BreakEventState (Variables|Default|GetEventState)))))
  (bind _result (Math|Integer|DecrementInt (Variables|Default|GeteventID))
    (:%20%20
      (Variables|Default|SeteventID _result)
      (CallFunction|UpdateEvent))))

(fn LLoadNext
  (Development|PrintString "Loading Next !")
  (Variables|Default|SetEventState (Utilities|Struct|MakeEventState (.ShowTracks (Utilities|Struct|BreakEventState (Variables|Default|GetEventState))) (.ShowJets (Utilities|Struct|BreakEventState (Variables|Default|GetEventState))) (.ShowClusters (Utilities|Struct|BreakEventState (Variables|Default|GetEventState))) (.AutoReload (Utilities|Struct|BreakEventState (Variables|Default|GetEventState))) (.ChangeToPreviousEvent (Utilities|Struct|BreakEventState (Variables|Default|GetEventState))) true))
  (bind _result (Math|Integer|IncrementInt (Variables|Default|GeteventID))
    (:%20%20
      (Variables|Default|SeteventID _result)
      (CallFunction|UpdateEvent))))

(fn DrawEvent
  (bind _eventstate (Variables|Default|GetEventState))
  (bind (_showtracks _showjets _showclusters) (Utilities|Struct|BreakEventState _eventstate))
  (Development|PrintString "DRAW EVENT CALLED")
  (bind _returnvalue (Class|Event|GetEventNr))
  (Rendering|Components|TextRender|SetText (Variables|Default|GetEventNumberDisplay) (Utilities|Text|ToText(Integer) _returnvalue false))
  (bind _returnvalue_2 (Class|Event|GetRunNr))
  (Rendering|Components|TextRender|SetText (Variables|Default|GetRunNumberDisplay) (Utilities|Text|ToText(Integer) _returnvalue_2 false))
  (if _showclusters
    (CallFunction|ShowClusters))
  (if _showtracks
    (CallFunction|ShowTracks)))

(fn UpdateEvent
  (CallFunction|ClearPreviousEvent)
  (Class|Event|GetEvent)
  (Audio|PlaySoundatLocation "/Game/StarterContent/Audio/clong.clong" "0, 0, 0"))

(fn ClearPreviousEvent)

(fn ShowTracks
  (bind _vertices (Variables|Default|GetVertices))
  (bind _triangles (Variables|Default|GetTriangles))
  (Class|Event|ShowTracksFunc)
  (Class|ProceduralMeshComponent|CreateMeshSection (Variables|Default|GetTrackComponent) 0 _vertices _triangles 0 0 0 0 false)
  (Rendering|Material|SetMaterial (Variables|Default|GetTrackComponent) 0 "/Game/Materials/M_Metal_Orange.M_Metal_Orange")
  (Development|PrintString (Utilities|String|Append "FINAL Vertices: " (Utilities|String|ToString(Integer) (Utilities|Array|Length _vertices)) "    Triangles:  " (Utilities|String|ToString(Integer) (Utilities|Array|Length _triangles)))))