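; Event submenu Blueprint with 3D buttons that toggle tracks, jets and clusters and control event playback on an EventBP actor.
; A Pointer overlap highlights the touched button with an emissive material, plays a sound and stores its object name as the current selection.
; MakeTheChange switches on that name to call the first EventBP found, while PressButton nudges toggle buttons in or out based on their relative X position.
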(event OnComponentBeginOverlap(Pointer)
  (params (OtherActor :type Actor%20Object%20Reference) (OtherComp :type Primitive%20Component%20Object%20Reference) (OtherBodyIndex :type Integer) (bFromSweep :type Boolean) (SweepResult :type Hit%20Result%20Structure%20%28by%20ref%29))
  (bind _returnvalue (Utilities|GetObjectName OtherComp))
  (Rendering|Material|SetMaterial OtherComp 2 "/Game/Materials/M_Metal_ChromeEmissive.M_Metal_ChromeEmissive")
  (Variables|Default|SetCurrentSelection _returnvalue)
  (Development|PrintString (Utilities|String|Append "event menu selected cube  " _returnvalue) false true "(R=0.000000,G=0.660000,B=1.000000,A=1.000000)" 2e+01)
  (Audio|PlaySoundatLocation "/Game/StarterContent/Audio/highlight.highlight" (Transformation|GetActorLocation) "0, 0, 0" 0.2))

(event OnComponentEndOverlap(Pointer)
  (params (OtherActor :type Actor%20Object%20Reference) (OtherComp :type Primitive%20Component%20Object%20Reference) (OtherBodyIndex :type Integer))
  (Rendering|Material|SetMaterial OtherComp 2 "/Game/Materials/M_Metal_Chrome.M_Metal_Chrome"))

(fn ConstructionScript)

(fn MaketheChange
  (bind _currentselection (Variables|Default|GetCurrentSelection))
  (Development|PrintString _currentselection)
  (bind _outactors (Actor|GetAllActorsOfClass "/Game/BPs/Events/EventBP.EventBP_C"))
  (Variables|Default|SetEvent (Utilities|Array|Get(acopy) _outactors))
  (switch string _currentselection
    (:Default
      (Development|PrintString "NothingSelected" false))
    (:Tracks
      (CallFunction|PressButton (Variables|Default|GetTracks))
      (Default|ToggleTracks (Variables|Default|GetEvent)))
    (:Jets
      (CallFunction|PressButton (Variables|Default|GetJets))
      (Default|ToggleJets (Variables|Default|GetEvent)))
    (:Clusters
      (CallFunction|PressButton (Variables|Default|GetClusters))
      (Default|ToggleClusters (Variables|Default|GetEvent)))
    (:REV
      (Default|LoadPrevious (Variables|Default|GetEvent)))
    (:PLAY
      (CallFunction|PressButton (Variables|Default|GetPLAY) :!label _label)
      (CallFunction|PressButton (Variables|Default|GetSTOP))
      (Default|ToggleAutoLoad (Variables|Default|GetEvent)))
    (:STOP
      (goto _label))
    (:FFW
      (Default|LoadNext (Variables|Default|GetEvent)))))

(fn PressButton
  (params (Button :type Static%20Mesh%20Component%20Object%20Reference))
  (if (> (.X (Math|Vector|BreakVector (.Location (Math|Transform|BreakTransform (Transformation|GetRelativeTransform Button))))) 2.0)
    ;[1 1 1] was pressed.. unpress it
    (Transformation|AddRelativeLocation Button "-5.000000, 0, 0" false false)
    (else
      (Transformation|AddRelativeLocation Button "5.000000, 0, 0" false false))))