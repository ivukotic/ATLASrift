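; VR flying pawn for a detector exhibit, with head-driven menus for a narrated tour, subdetector selection and event selection.
; A Level state machine advances on MainMenu presses, while Tick rotates or slides the active menu by headset rotation delta.
; Selections derive from menu yaw or offset; the tour moves the pawn along a timeline.
; Subdetectors, found by tag, can be shown or hidden; other manipulation options and event selection are stubs.
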(event EventTick
  (params (DeltaSeconds :type Float%20%28single-precision%29))
  (switch int (Variables|Default|Getlevel)
    (:1
      (CallFunction|RunMainMenu))
    (:2
      (CallFunction|RunDetectorSubMenu))
    (:3
      (CallFunction|RunSubDetectorManipulation))
    (:4
      (CallFunction|RunEventSubMenu))))

(event Input|ActionEvents|InputActionbackMenu
  (:Pressed
    (CallFunction|AllReset)
    (Development|PrintString "Full menu reset" false)
    (Audio|Components|Audio|Stop (Variables|Default|GetGuideVoiceComponent))
    (bind _locationtrack (Timeline|TourTimeline Stop)
      (:Update
        (Transformation|SetActorLocation (Game|Player|GetPlayerPawn 0) _locationtrack false))
      (:EventsAlongTrack
        (Default|CallTimeLineDispatch (Variables|Default|GeteventCounter))
        (Variables|Default|SeteventCounter (+ (Variables|Default|GeteventCounter) 1))))))

(event Input|ActionEvents|InputActionMainMenu
  (bind _mm (Variables|Default|GetMM))
  (bind _submenu_detector (Variables|Default|Getsubmenu-detector))
  (bind _relativerotation (Variables|/Script/Engine.SceneComponent|GetRelativeRotation _submenu_detector))
  (bind _relativerotation_2 (Variables|/Script/Engine.SceneComponent|GetRelativeRotation _mm))
  (bind _yaw (Class|KismetMathLibrary|BreakRot _relativerotation_2))
  (bind _yaw_2 (Class|KismetMathLibrary|BreakRot _relativerotation))
  (bind _returnvalue (+ 190.588235 _yaw_2))
  (bind _returnvalue_2 (+ 225.0 _yaw))
  (bind _returnvalue_3 (Math|Float|Division(WholeandRemainder) _returnvalue_2 9e+01))
  (bind _returnvalue_4 (Math|Float|Division(WholeandRemainder) _returnvalue 21.17647))
  (:Pressed
    (switch int (Variables|Default|Getlevel)
      (:0
        (Variables|Default|Setlevel 1)
        (CallFunction|EnableMainMenu))
      (:1
        (Variables|Default|Setlevel 2)
        (Development|PrintString (Utilities|String|ToString(Integer) _returnvalue_3) false)
        ;[1 1 1] 0|4- tour 1-detector 2-event 3 - about
        (switch int _returnvalue_3
          (:0
            (CallFunction|AllReset :!label _label)
            (Audio|Components|Audio|Play (Variables|Default|GetGuideVoiceComponent) 0.0)
            (bind _locationtrack (Timeline|TourTimeline PlayFromStart)
              (:Update
                (Transformation|SetActorLocation (Game|Player|GetPlayerPawn 0) _locationtrack false))
              (:EventsAlongTrack
                (Default|CallTimeLineDispatch (Variables|Default|GeteventCounter))
                (Variables|Default|SeteventCounter (+ (Variables|Default|GeteventCounter) 1)))))
          (:1
            (CallFunction|EnableDetectorSubMenu))
          (:2
            (CallFunction|AllReset)
            (Variables|Default|Setlevel 4)
            (CallFunction|EnableEventSubMenu))
          (:3
            (CallFunction|AllReset))
          (:4
            (goto _label))))
      (:2
        (Variables|Default|Setlevel 3)
        (CallFunction|HandleSubdetSelection))
      (:3
        (CallFunction|HandleSubdetManipSelection))
      (:4
        (Variables|Default|Setlevel 5)
        (Variables|Default|SetselectedOption _returnvalue_4)
        (Development|PrintString (Utilities|String|ToString(Integer) _returnvalue_4) false)
        (CallFunction|AllReset)))))

(event Input|AxisEvents|InputAxisMoveUp
  (params (AxisValue :type Float%20%28single-precision%29))
  (Transformation|SetActorLocation (+ (Math|Vector|MakeVector 0.0 0.0 AxisValue) (Transformation|GetActorLocation)) false))

(fn ConstructionScript)

(fn AllReset
  (Variables|Default|Setlevel 0)
  (Variables|Default|SetselectedOption 0)
  (Rendering|SetVisibility false true)
  (Rendering|SetVisibility false true)
  (Rendering|SetVisibility false true)
  (Rendering|SetVisibility false true)
  (Rendering|SetVisibility (Variables|Default|GetHeadLamp) false false))

(fn RunMainMenu
  (bind _devicerotation (Class|HeadMountedDisplayFunctionLibrary|GetOrientationandPosition))
  (bind _baserotation (Variables|Default|GetBaseRotation))
  (bind _returnvalue (Math|Rotator|Delta(Rotator) _devicerotation _baserotation))
  (bind _returnvalue_2 (* _returnvalue 0.1))
  (bind _yaw (Class|KismetMathLibrary|BreakRot _returnvalue_2))
  (if (Variables|/Script/Engine.SceneComponent|GetbVisible (Variables|Default|GetMM))
    (if (> (Math|Float|Absolute(Float) _yaw) 0.1)
      (Transformation|AddRelativeRotation (Variables|Default|GetMM) (Class|KismetMathLibrary|MakeRot 0.0 _yaw 0.0) false))))

(fn EnableMainMenu
  (CallFunction|LoadConfig)
  (Rendering|SetVisibility (Variables|Default|GetMM) true false)
  (Rendering|SetVisibility (Variables|Default|GetHeadLamp) true false)
  (Variables|Default|SetBaseRotation (.DeviceRotation (Class|HeadMountedDisplayFunctionLibrary|GetOrientationandPosition)))
  (Audio|PlaySoundatLocation "/Game/Audio/Woosh-Mark_DiAngelo-4778593.Woosh-Mark_DiAngelo-4778593" (Transformation|GetActorLocation) (Variables|/Game/Maps/MySaveData.MySaveData_C|GetsoundEfffectsVolume (Variables|Default|GetCurrSettings)))
  (Development|PrintString "Activated Main Menu" false))

(fn RunDetectorSubMenu
  (bind _devicerotation (Class|HeadMountedDisplayFunctionLibrary|GetOrientationandPosition))
  (bind _baserotation (Variables|Default|GetBaseRotation))
  (bind _returnvalue (Math|Rotator|Delta(Rotator) _devicerotation _baserotation))
  (bind _returnvalue_2 (* _returnvalue 0.1))
  (bind _yaw (Class|KismetMathLibrary|BreakRot _returnvalue_2))
  (if (Variables|/Script/Engine.SceneComponent|GetbVisible (Variables|Default|Getsubmenu-detector))
    (if (> (Math|Float|Absolute(Float) _yaw) 0.1)
      (Transformation|AddLocalRotation (Variables|Default|Getsubmenu-detector) (Class|KismetMathLibrary|MakeRot 0.0 _yaw 0.0) false))))

(fn EnableDetectorSubMenu
  (Rendering|SetVisibility (Variables|Default|GetMM) false false)
  (Rendering|SetVisibility true true)
  (Variables|Default|SetBaseRotation (.DeviceRotation (Class|HeadMountedDisplayFunctionLibrary|GetOrientationandPosition)))
  (Audio|PlaySoundatLocation "/Game/Audio/Woosh-Mark_DiAngelo-4778593.Woosh-Mark_DiAngelo-4778593" (Transformation|GetActorLocation))
  (Development|PrintString "Activated Detector Sub Menu" false))

(fn EnableSubDetectorManipulation
  (Rendering|SetVisibility false true)
  (Rendering|SetVisibility true true)
  (Variables|Default|SetBaseRotation (.DeviceRotation (Class|HeadMountedDisplayFunctionLibrary|GetOrientationandPosition)))
  (Audio|PlaySoundatLocation "/Game/Audio/Woosh-Mark_DiAngelo-4778593.Woosh-Mark_DiAngelo-4778593" (Transformation|GetActorLocation) 0.0)
  (Development|PrintString "Activated Sub Detector Manipulation" false))

(fn RunSubDetectorManipulation
  (bind _devicerotation (Class|HeadMountedDisplayFunctionLibrary|GetOrientationandPosition))
  (bind _baserotation (Variables|Default|GetBaseRotation))
  (bind _returnvalue (Math|Rotator|Delta(Rotator) _devicerotation _baserotation))
  (bind _returnvalue_2 (* _returnvalue 2.0))
  (bind _pitch (Class|KismetMathLibrary|BreakRot _returnvalue_2))
  ;[1 1 1] unneeded
  (if (Variables|/Script/Engine.SceneComponent|GetbVisible (Variables|Default|Getsubdetmanip))
    (if (> (Math|Float|Absolute(Float) _pitch) 0.1)
      (Transformation|SetRelativeLocation (Components|GetChildComponent (Components|GetChildComponent (Variables|Default|Getsubdetmanip) 0) 2) (Math|Vector|MakeVector 0.0 0.0 _pitch) false))))

(fn EnableEventSubMenu
  (Rendering|SetVisibility true true)
  (Variables|Default|SetBaseRotation (.DeviceRotation (Class|HeadMountedDisplayFunctionLibrary|GetOrientationandPosition)))
  (Audio|PlaySoundatLocation "/Game/Audio/Woosh-Mark_DiAngelo-4778593.Woosh-Mark_DiAngelo-4778593" (Transformation|GetActorLocation))
  (Development|PrintString "Activated Sub Menu Event" false))

(fn RunEventSubMenu
  (bind _devicerotation (Class|HeadMountedDisplayFunctionLibrary|GetOrientationandPosition))
  (bind _baserotation (Variables|Default|GetBaseRotation))
  (bind _returnvalue (Math|Rotator|Delta(Rotator) _devicerotation _baserotation))
  (bind _returnvalue_2 (* _returnvalue 3.0))
  (bind (_pitch _yaw) (Class|KismetMathLibrary|BreakRot _returnvalue_2))
  ;[1 1 1] unneeded
  (if (Variables|/Script/Engine.SceneComponent|GetbVisible (Variables|Default|Getsubmenu-event))
    (if (or (> (Math|Float|Absolute(Float) _pitch) 0.1) (> (Math|Float|Absolute(Float) _yaw) 0.1))
      (Transformation|SetRelativeLocation (Components|GetChildComponent (Components|GetChildComponent (Variables|Default|Getsubmenu-event) 0) 1) (Math|Vector|MakeVector 0.0 _yaw _pitch) false))))

(fn LoadConfig
  (bind _returnvalue (SaveGame|DoesSaveGameExist "mySettings"))
  (if _returnvalue
    (bind _returnvalue_2 (SaveGame|LoadGamefromSlot "mySettings"))
    (bind _asmy_save_data (Utilities|Casting|CastToMySaveData _returnvalue_2))
    (bind _output_get (Variables|Default|SetCurrSettings _asmy_save_data))
    (Audio|Components|Audio|AdjustVolume (Variables|Default|GetGuideVoiceComponent) 0.0 (Variables|/Game/Maps/MySaveData.MySaveData_C|GetsoundSpeachVolume _output_get) :!class /Script/Engine.AudioComponent)))

(fn RunSubdetectorTour
  (params (sebdet :type Actor%20Object%20Reference))
  (Development|PrintString (Utilities|GetObjectName sebdet)))

(fn HandleSubdetManipSelection
  (bind _subdetmanip (Variables|Default|Getsubdetmanip))
  (bind _returnvalue (Components|GetChildComponent _subdetmanip 0))
  (bind _returnvalue_2 (Components|GetChildComponent _returnvalue 2))
  (bind _relativelocation (Variables|/Script/Engine.SceneComponent|GetRelativeLocation _returnvalue_2))
  (bind _z (Math|Vector|BreakVector _relativelocation))
  (bind _returnvalue_3 (+ 62.0 _z))
  (bind _returnvalue_4 (Math|Float|Division(WholeandRemainder) _returnvalue_3 25.0))
  (Development|PrintString (Utilities|String|Append "SELECTED  manip panel INDEX" (Utilities|String|ToString(Integer) _returnvalue_4)) false)
  (bind _outactors (Actor|GetAllActorsOfClass "/Script/Engine.Actor"))
  (for _array_element _outactors
    (if (> (Utilities|Array|Length (Variables|/Script/Engine.Actor|GetTags _array_element)) 0)
      (if (Utilities|Name|Equal(Name) (Utilities|Array|Get(acopy) (Variables|/Script/Engine.Actor|GetTags _array_element)) (Utilities|String|StringToName (Utilities|String|ToString(Integer) (Variables|Default|GetselectedOption))))
        (Variables|Default|SetSelectedSubDet _array_element)
        (Development|PrintString (Utilities|String|Append "Selected Subdetector:  " (Utilities|GetDisplayName (Variables|Default|GetSelectedSubDet))) false)
        (switch int _returnvalue_4
          (:0
            (Development|PrintString "Tour")
            (CallFunction|RunSubdetectorTour (Variables|Default|GetSelectedSubDet)))
          (:1
            (Development|PrintString "Gallery"))
          (:2
            (Development|PrintString "Visible")
            (Rendering|SetActorHiddenInGame (Variables|Default|GetSelectedSubDet) false))
          (:3
            (Development|PrintString "Invisible")
            (Rendering|SetActorHiddenInGame (Variables|Default|GetSelectedSubDet) true))
          (:4
            (Development|PrintString "Translcent")))))))

(fn HandleSubdetSelection
  (bind _submenu_detector (Variables|Default|Getsubmenu-detector))
  (bind _relativerotation (Variables|/Script/Engine.SceneComponent|GetRelativeRotation _submenu_detector))
  (bind _yaw (Class|KismetMathLibrary|BreakRot _relativerotation))
  (bind _returnvalue (+ 190.588235 _yaw))
  (bind _returnvalue_2 (Math|Float|Division(WholeandRemainder) _returnvalue 21.17647))
  (Variables|Default|SetselectedOption _returnvalue_2)
  (Development|PrintString (Utilities|String|Append "                               SELECTED SUBDET............................................................:" (Utilities|String|ToString(Integer) _returnvalue_2)))
  (CallFunction|EnableSubDetectorManipulation))