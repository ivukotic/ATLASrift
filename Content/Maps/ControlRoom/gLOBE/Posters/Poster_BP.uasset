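; Poster actor that displays a supplied material and can carry an audio clip, toggled by hits on the poster mesh.
; SetPoster scales the mesh from a ratio and Surface value, applies the material and reveals it; SetAudioAsset assigns the sound and reveals the Sign.
; While the Sign is visible, each hit plays, pauses or resumes the audio, swapping the Sign between HasAudio and Playing materials.
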(event OnComponentHit(PosterMesh)
  (params (HitComponent :type Primitive%20Component%20Object%20Reference) (OtherActor :type Actor%20Object%20Reference) (OtherComp :type Primitive%20Component%20Object%20Reference) (NormalImpulse :type Vector :default "0, 0, 0") (Hit :type Hit%20Result%20Structure%20%28by%20ref%29))
  (bind _audio (Variables|Default|GetAudio))
  (Development|PrintString (Utilities|GetObjectName OtherActor))
  (if (not (Variables|/Script/Engine.SceneComponent|GetbHiddenInGame (Variables|Default|GetSign)))
    (if (Audio|Components|Audio|IsPlaying (Variables|Default|GetAudio))
      (Class|AudioComponent|SetPaused _audio true)
      (Variables|Default|SetPaused true)
      (Rendering|Material|SetMaterial (Variables|Default|GetSign) 0 (Variables|Default|GethasAudio))
      (else
        (if (Variables|Default|GetPaused)
          (Class|AudioComponent|SetPaused _audio false)
          (Variables|Default|SetPaused false)
          (else
            (Audio|Components|Audio|Play _audio 0.0)))
        (Rendering|Material|SetMaterial (Variables|Default|GetSign) 0 (Variables|Default|Getplaying))))))

(event EventBeginPlay)

(event Collision|EventActorBeginOverlap
  (params (OtherActor :type Actor%20Object%20Reference)))

(event EventTick
  (params (DeltaSeconds :type Float%20%28single-precision%29)))

(fn ConstructionScript
  (Rendering|Material|SetMaterial (Variables|Default|GetSign) 0 (Variables|Default|GethasAudio)))

(fn SetAudioAsset
  (params (SoundAsset :type Sound%20Base%20Object%20Reference))
  (Audio|Components|Audio|SetSound (Variables|Default|GetAudio) SoundAsset)
  (Development|SetHiddeninGame (Variables|Default|GetSign) false false))

(fn SetPoster
  (params (PosterMaterial :type Material%20Object%20Reference) (ratio :type Float%20%28single-precision%29))
  (bind _postermesh (Variables|Default|GetPosterMesh))
  (bind _surface (Variables|Default|GetSurface))
  (bind _returnvalue (/ _surface ratio))
  (Transformation|SetWorldScale3D _postermesh (Math|Vector|MakeVector (/ _surface _returnvalue) _returnvalue 0.0))
  (Rendering|Material|SetMaterial _postermesh 0 PosterMaterial)
  (Development|SetHiddeninGame (Variables|Default|GetPosterMesh) false false))