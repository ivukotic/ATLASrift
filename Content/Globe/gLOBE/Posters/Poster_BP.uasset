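; Poster actor that shows an image, optionally with an audio track or a video, and plays it while the player's flying character is nearby.
; Initialize sets the poster material, aspect scale and media, hiding the status sign on posters without media.
; TriggerBox overlaps, filtered by the "FlyingCharacter" display name, call Start and Pause.
; These drive the audio component or streaming media player, swapping screen and sign materials, with video taking priority over audio.
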(event OnComponentBeginOverlap(TriggerBox)
  (params (OverlappedComponent :type Primitive%20Component%20Object%20Reference) (OtherActor :type Actor%20Object%20Reference) (OtherComp :type Primitive%20Component%20Object%20Reference) (OtherBodyIndex :type Integer) (bFromSweep :type Boolean) (SweepResult :type Hit%20Result%20Structure%20%28by%20ref%29))
  ;[1 1 1] start
  (if (Utilities|Enum|Equal(Enum) (Utilities|GetDisplayName OtherActor) "FlyingCharacter")
    (CallFunction|Start)))

(event OnComponentEndOverlap(TriggerBox)
  (params (OverlappedComponent :type Primitive%20Component%20Object%20Reference) (OtherActor :type Actor%20Object%20Reference) (OtherComp :type Primitive%20Component%20Object%20Reference) (OtherBodyIndex :type Integer))
  ;[1 1 1] Stop overlap
  (if (Utilities|Enum|Equal(Enum) (Utilities|GetDisplayName OtherActor) "FlyingCharacter")
    (CallFunction|Pause)))

(fn ConstructionScript)

(fn TogglePlayingSign
  (params (play :type Boolean))
  (bind _sign (Variables|Default|GetSign))
  (if play
    (Rendering|Material|SetMaterial _sign 0 "/Game/Globe/gLOBE/Posters/playing_Mat.playing_Mat")
    (else
      (Rendering|Material|SetMaterial _sign 0 "/Game/Globe/gLOBE/Posters/not_playing_Mat.not_playing_Mat"))))

(fn Initialize
  (params (Poster :type Material%20Object%20Reference) (Aspect :type Float%20%28single-precision%29) (isAudio :type Boolean) (Audio :type Sound%20Base%20Object%20Reference) (isVideo :type Boolean) (Video :type Stream%20Media%20Source%20Object%20Reference))
  (bind _postermesh (Variables|Default|GetPosterMesh))
  (Utilities|FlowControl|Sequence
    (:then_0
      ;[1 1 1] Audio Supported Poster
      (bind _output_get (Variables|Default|SetisAudio isAudio))
      (if _output_get
        (Audio|Components|Audio|SetSound (Variables|Default|GetAudio) Audio)))
    (:then_1
      ;[1 1 1] Video
      (bind _output_get_2 (Variables|Default|SetisVideo isVideo))
      (if _output_get_2
        (Rendering|Material|SetMaterial (Variables|Default|GetPosterMesh) 0 "/Game/HandMenu/Pause_screen_Mat.Pause_screen_Mat")
        (Variables|Default|SetVideo Video)))
    (:then_2
      ;[1 1 1] Set Sign
      (Development|SetHiddeninGame (Variables|Default|GetSign) (not (or isAudio isVideo)) false))
    (:then_3
      ;[1 1 1] Poster
      (if (not isVideo)
        (Rendering|Material|SetMaterial _postermesh 0 Poster)
        (Transformation|SetWorldScale3D _postermesh (Math|Vector|MakeVector 1.2 Aspect 0.0))))))

(fn Start
  (bind _streamingmediaplayer (Variables|Default|GetStreamingMediaPlayer))
  (Development|PrintString "Start overlap")
  ;[1 1 1] Audio or Video?
  (if (Variables|Default|GetisVideo)
    ;[1 1 1] Starting video
    (Rendering|Material|SetMaterial (Variables|Default|GetPosterMesh) 0 "/Game/Audio/StreamingMediaPlayer_Video_Mat.StreamingMediaPlayer_Video_Mat")
    (if (Audio|Components|Audio|IsPlaying _streamingmediaplayer)
      (Media|MediaPlayer|Play _streamingmediaplayer :!class /Script/MediaAssets.MediaPlayer)
      (Development|PrintString "Continued ")
      (CallFunction|TogglePlayingSign true :!label _label)
      (else
        (bind _returnvalue (Media|MediaPlayer|OpenSource _streamingmediaplayer (Variables|Default|GetVideo)))
        (if _returnvalue
          (Development|PrintString "Media successfully opened.")
          (goto _label)
          (else
            (Development|PrintString "Media could not be opened!!!" true true "(R=1.000000,G=0.000000,B=0.058392,A=1.000000)" 1e+01)))))
    (elif (Variables|Default|GetisAudio)
      ;[1 1 1] Audio start or restart
      (if (Audio|Components|Audio|IsPlaying (Variables|Default|GetAudio))
        ;;[1 1 1] continue
        (Class|AudioComponent|SetPaused (Variables|Default|GetAudio) false)
        (Development|PrintString "Continued ")
        (else
          (Audio|Components|Audio|Play (Variables|Default|GetAudio) 0.0)))
      (CallFunction|TogglePlayingSign true))))

(fn Pause
  ;[1 1 1] Audio or Video?
  (Development|PrintString "Exit poster trigger.")
  (if (Variables|Default|GetisVideo)
    (Sequencer|Player|Pause (Variables|Default|GetStreamingMediaPlayer))
    (Rendering|Material|SetMaterial (Variables|Default|GetPosterMesh) 0 "/Game/HandMenu/Pause_screen_Mat.Pause_screen_Mat")
    (CallFunction|TogglePlayingSign false :!label _label)
    (elif (Variables|Default|GetisAudio)
      (Class|AudioComponent|SetPaused (Variables|Default|GetAudio) true)
      (goto _label))))